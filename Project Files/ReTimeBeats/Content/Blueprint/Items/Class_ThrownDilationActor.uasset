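; Throwable dilation item actor that can be picked up and thrown as a projectile.
; PickUp attaches it to the given actor, keeping world transform.
; Throw calls DetachFromActor on the attach parent rather than itself, then faces along that parent's forward vector.
; It then applies the configured speed and gravity values to ProjectileMovement and activates it; no time dilation logic appears here.
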(event `Throw`
  (bind _returnvalue (`self.GetAttachParentActor`))
  (bind _projectilemovement (`self.ProjectileMovement`))
  (`self.K2_DetachFromActor` _returnvalue "KeepWorld" "KeepWorld" "KeepWorld")
  (`self.K2_SetActorRotation` (`KismetMathLibrary.MakeRotFromX` (`self.GetActorForwardVector` _returnvalue)))
  (set `ProjectileMovementComponent.InitialSpeed` (`self.Thrown Speed`) _projectilemovement)
  (set `ProjectileMovementComponent.MaxSpeed` (`self.Max Speed`) _projectilemovement)
  (set `ProjectileMovementComponent.ProjectileGravityScale` (`self.Gravity Scale`) _projectilemovement)
  (`ActorComponent.SetActive` _projectilemovement true true))

(event `Pick Up`
  (params (Actor :type "Actor Object Reference"))
  (`self.K2_AttachToActor` Actor "None" "KeepWorld" "KeepWorld" "KeepWorld"))

(fn `UserConstructionScript`)